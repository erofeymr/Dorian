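; BP_inventory opens and closes the inventory screen and tracks whether it is open.
; ShowInventory creates a new WBP_inventory widget on each call, with the player pawn as outer, stores it and adds it to the viewport.
; HideInventory removes the stored widget from its parent and clears the open flag, provided the widget is valid.
; The event graph holds no logic.
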(fn `HideInventory`
  (`/Engine/EditorBlueprintResources/StandardMacros.IsValid` (`self.WBP_inventory`)
    (:`Is Valid`
      (`Widget.RemoveFromParent` (`self.WBP_inventory`))
      (set `self.IsInventoryOpen` false))))

(fn `ShowInventory`
  (set `self.IsInventoryOpen` true)
  (bind _returnvalue (`|GenericCreateObject` "/Game/Dorian/Inventory/WBP_inventory.WBP_inventory_C" (`GameplayStatics.GetPlayerPawn` 0)))
  (bind _output_get (set `self.WBP_inventory` _returnvalue))
  (`UserWidget.AddToViewport` _output_get 0))