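; BP_Di is a playable character Blueprint that provides camera controls and switching to the Dorian character.
; Pressing SpaceBar makes its controller possess the pawn held in the Dorian reference.
; Holding the unlock-camera input, noted as middle mouse, lets Turn and LookUp axes drive controller yaw and pitch.
; The CameraZoom wheel axis changes the spring arm length in steps within a clamped range.
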(event `Key|SpaceBar`
  (params (Key :type "Key Structure"))
  ;[1 1 1] Переключение между персонажами
  (:`Pressed`
    (`Controller.Possess` (`self.GetController`) (`self.Dorian`))))

(event `InputAction|unlock Camera`
  (params (Key :type "Key Structure"))
  ;[1 1 1] Поворот Камеры при нажатие средней кнопки мыши
  (:`Pressed`
    (set `self.UnlockCamera` true))
  (:`Released`
    (set `self.UnlockCamera` false)))

(event `InputAxis|LookUp`
  (params (AxisValue :type "Float (single-precision)"))
  ;[1 1 1] Поворот Камеры при нажатие средней кнопки мыши
  (if (`self.UnlockCamera`)
    (`self.AddControllerPitchInput` AxisValue)))

(event `InputAxis|Turn`
  (params (AxisValue :type "Float (single-precision)"))
  ;[1 1 1] Поворот Камеры при нажатие средней кнопки мыши
  (if (`self.UnlockCamera`)
    (`self.AddControllerYawInput` AxisValue)))

(event `InputAxis|CameraZoom`
  (params (AxisValue :type "Float (single-precision)"))
  (bind _springarm (`self.SpringArm`))
  ;[1 1 1] При использовании колеса мыши  камера  меняет свой зум
  (set `SpringArmComponent.TargetArmLength` (`KismetMathLibrary.FClamp` (- (`SpringArmComponent.TargetArmLength` _springarm) (* AxisValue (`self.CameraZoomStep`))) 300.0 1000.0) _springarm))

(fn `UserConstructionScript`)