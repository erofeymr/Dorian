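; Player controller for click-and-hold movement: the pawn follows the cursor while the Mouse Location input is held.
; That input opens and closes a gate on Tick, which traces under the cursor on the Visibility channel each frame.
; MovetoHitLocation then calls SimpleMoveToLocation toward the hit point, but only when it is at least MinDistance from the pawn.
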(event `self.ReceiveTick`
  (params (DeltaSeconds :type "Float (single-precision)"))
  ;[1 1 1] При зажатой левой кнопки мыши персонаж будет ходить  за курсором
  (`/Engine/EditorBlueprintResources/StandardMacros.Gate` true :!label _label
    (:`Exit`
      (`self.MovetoHitLocation` (`self.GetHitResultUnderCursorByChannel` "TraceTypeQuery1")))))

(event `InputAction|Mouse Location`
  (params (Key :type "Key Structure"))
  ;[1 1 1] При зажатой левой кнопки мыши персонаж будет ходить  за курсором
  (:`Pressed`
    (goto _label :!via `Open`))
  (:`Released`
    (goto _label :!via `Close`)))

(fn `MovetoHitLocation`
  (params (hit :type "HitResult Structure"))
  (bind (_bblockinghit _binitialoverlap _time _distance _location) (`GameplayStatics.BreakHitResult` hit))
  (if (>= (`KismetMathLibrary.VSize` (- (`self.K2_GetActorLocation` (`self.K2_GetPawn`)) _location)) (`self.MinDistance`))
    (`AIBlueprintHelperLibrary.SimpleMoveToLocation` self _location)))

(fn `UserConstructionScript`)