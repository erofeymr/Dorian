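; BP_Dorian is the playable Dorian character, handling character switching and camera rotation.
; Pressing Space makes its controller possess the MinionDi reference, handing control to that character.
; Holding the camera unlock input (middle mouse button) sets UnlockCamera, which gates the Turn and LookUp axes feeding controller yaw and pitch.
; The CameraZoom axis event and the construction script are empty.
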(event `Key|SpaceBar`
  (params (Key :type "Key Structure"))
  ;[1 1 1] Переключение персонажей
  (:`Pressed`
    (`Controller.Possess` (`self.GetController`) (`self.MinionDi`))))

(event `InputAction|unlock Camera`
  (params (Key :type "Key Structure"))
  ;[1 1 1] Поворот Камеры при нажатие средней кнопки мыши
  (:`Pressed`
    (set `self.UnlockCamera` true))
  (:`Released`
    (set `self.UnlockCamera` false)))

(event `InputAxis|LookUp`
  (params (AxisValue :type "Float (single-precision)"))
  ;[1 1 1] Поворот Камеры при нажатие средней кнопки мыши
  (if (`self.UnlockCamera`)
    (`self.AddControllerPitchInput` AxisValue)))

(event `InputAxis|Turn`
  (params (AxisValue :type "Float (single-precision)"))
  ;[1 1 1] Поворот Камеры при нажатие средней кнопки мыши
  (if (`self.UnlockCamera`)
    (`self.AddControllerYawInput` AxisValue)))

(event `InputAxis|CameraZoom`
  (params (AxisValue :type "Float (single-precision)")))

(fn `UserConstructionScript`)